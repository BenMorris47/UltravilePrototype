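; BP_CameraCollider is a trigger volume that ties a CineCamera to units entering its Box.
; On overlap, it registers itself as the BP_Unit's CurrentCamera and, if that unit is selected, calls SwitchCamera.
; The SwitchCamera event tells player 0's BP_CameraPawn to switch to this collider's CineCamera.
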(event OnComponentBeginOverlap(Box)
  (params (OverlappedComponent :type Primitive%20Component%20Object%20Reference) (OtherActor :type Actor%20Object%20Reference) (OtherComp :type Primitive%20Component%20Object%20Reference) (OtherBodyIndex :type Integer) (bFromSweep :type Boolean) (SweepResult :type Hit%20Result%20Structure%20%28by%20ref%29))
  (bind _asbp_unit (Utilities|Casting|CastToBP_Unit OtherActor))
  (Variables|/Game/Units/BP_Unit.BP_Unit_C|SetCurrent%20Camera _asbp_unit self)
  (if (Variables|/Game/Units/BP_Unit.BP_Unit_C|GetisSelected _asbp_unit)
    (CallFunction|SwitchCamera)))

(event Custom|Switch%20Camera
  (bind _asbp_camera_pawn (Utilities|Casting|CastToBP_CameraPawn (Game|Player|GetPlayerPawn 0)))
  (Default|SwitchCamera _asbp_camera_pawn (Variables|Default|GetCineCamera)))

(fn ConstructionScript)