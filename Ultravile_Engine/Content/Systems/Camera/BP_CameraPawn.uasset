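; BP_CameraPawn is a pawn with a cine camera that moves between camera positions and aims at a target.
; SwitchCamera stores the camera's current transform, then a timeline lerps it to the new camera's transform and prints a debug message when done.
; Tick rotates the camera to look at Target whenever it is valid, with ticking explicitly enabled after a short delay following BeginPlay.
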(event Custom|Switch%20Camera
  (params (New%20Camera :type Cine%20Camera%20Component%20Object%20Reference))
  (Variables|Default|SetcameraPreMoveTransform (Transformation|GetWorldTransform (Variables|Default|GetCineCamera)))
  (bind _lerp (Timeline|Timeline_0 PlayFromStart)
    (:Update
      (Transformation|SetWorldTransform (Variables|Default|GetCineCamera) (Math|Transform|Lerp(Transform) (Variables|Default|GetcameraPreMoveTransform) (Transformation|GetWorldTransform New%20Camera) _lerp) false false))
    (:Finished
      (Development|PrintString "Cam Done"))))

(event EventTick
  (params (DeltaSeconds :type Float%20%28single-precision%29))
  (bind _target (Variables|Default|GetTarget))
  (Utilities|IsValid _target
    (:Is%20Valid
      (Transformation|SetWorldRotation (Variables|Default|GetCineCamera) (Math|Rotator|FindLookatRotation (Transformation|GetWorldLocation (Variables|Default|GetCineCamera)) (Transformation|GetActorLocation _target)) false false))))

(event EventBeginPlay
  (Utilities|FlowControl|Delay 2.0)
  (Actor|Tick|SetActorTickEnabled true))

(fn ConstructionScript)