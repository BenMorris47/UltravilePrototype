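; Card manager for a grid-based tactics game, running the selected unit's hand of pip-costed cards.
; Hand entries map GUIDs to names in a card dictionary, with debug keys for JSON save and load.
; Selecting a card shows castable cells through a Dijkstra flood fill filtered by target type.
; Using one applies damage or healing, spends pips and spawns effects, while event dispatchers broadcast hand, selection and affordability changes.
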(event Custom|UnitPipsUpdated
  (params (currentPipAmount :type Integer))
  (CallFunction|CheckCardAvalibility currentPipAmount))

(event Custom|BindUnitPipsUpdated
  (params (Unit :type BP%20Unit%20Object%20Reference))
  (EventDispatchers|BindEventtoPipsUpdated Unit (delegate Custom|UnitPipsUpdated)))

(event Custom|UnbindUnitPipsUpdated
  (params (Unit :type BP%20Unit%20Object%20Reference))
  (EventDispatchers|UnbindEventfromPipsUpdated Unit (delegate Custom|UnitPipsUpdated)))

(event EventBeginPlay
  (bind _returnvalue (Actor|GetActorOfClass "/Game/Systems/Grid/BP_GridManagerDataVersion.BP_GridManagerDataVersion_C"))
  (Variables|Default|SetGridManager _returnvalue)
  (bind _returnvalue_2 (Game|SpawnActorfromClass "/Game/Systems/CardSystem/CardParticleAndSoundController.CardParticleAndSoundController_C" (Math|Transform|MakeTransform "0, 0, 0" "0, 0, 0" "1.000000,1.000000,1.000000") "Undefined" 0 0))
  (Variables|Default|SetCardParticalAndSoundManager _returnvalue_2))

(event Input|KeyboardEvents|B
  (params (Key :type Key%20Structure))
  (:Pressed
    (bind (_outsuccess _outinfomessage) (Class|CardManager|WriteCardStructtoJson (Utilities|String|Append (Class|SomnusToolsLibrary|GetContentDir) "Data\\CardData\\" "CardData.Json") (Utilities|Struct|MakeCardDictionaryStruct (Variables|Default|GetCardDictionary))))
    (Development|PrintString _outinfomessage true true (Math|Color|SelectColor "(R=0.192786,G=0.011236,B=0.953125,A=1.000000)" "(R=0.968750,G=0.135355,B=0.000000,A=1.000000)" _outsuccess))))

(event Input|KeyboardEvents|V
  (params (Key :type Key%20Structure))
  (:Pressed
    (bind (_outsuccess _outinfomessage _returnvalue) (Class|CardManager|ReadCardStructfromJson (Utilities|String|Append (Class|SomnusToolsLibrary|GetContentDir) "Data\\CardData\\" "CardData.Json")))
    (Development|PrintString _outinfomessage true true (Math|Color|SelectColor "(R=0.192786,G=0.011236,B=0.953125,A=1.000000)" "(R=0.968750,G=0.135355,B=0.000000,A=1.000000)" _outsuccess))
    (bind _output_get (Variables|Default|SetCardDictionary (Utilities|Struct|BreakCardDictionaryStruct _returnvalue)))
    (bind _keys (Utilities|Map|Keys _output_get))
    (CallFunction|LoadHand _keys true)))

(fn ConstructionScript)

(fn LoadHand
  (params (CardsToLoad :type Array%20of%20Strings) (ClearOldHand :type Boolean))
  (if ClearOldHand
    (CallFunction|ClearHand))
  (for _array_element CardsToLoad
    (CallFunction|AddCard _array_element false))
  (Default|CallLoadHandEvent (Variables|Default|GetCardsInHand)))

(fn ClearHand
  (if (Guid|IsValidGuid (Variables|Default|GetSelectedCard))
    (CallFunction|DeselectCard (Variables|Default|GetSelectedCard) false))
  (bind _keys (Utilities|Map|Keys (Variables|Default|GetCardsInHand)))
  (for _array_element _keys
    (CallFunction|RemoveCard _array_element false))
  (Default|CallClearHandEvent)
  (Utilities|Map|Clear (Variables|Default|GetCardsInHand)))

(fn SelectCard
  (params (cardGuid :type Guid%20Structure))
  (if (not (== cardGuid (Variables|Default|GetSelectedCard)))
    (if (>= (Variables|/Game/Units/BP_Unit.BP_Unit_C|GetcurrentActionPips (Variables|Default|GetCurrentUnit)) (.pipcost (CallFunction|CardGuidtoData cardGuid)))
      (CallFunction|DeselectCard (Variables|Default|GetSelectedCard) false)
      (Default|ToggleMovemode (Variables|Default|GetGridManager) false)
      (CallFunction|DisplayCardRange cardGuid)
      (bind _output_get (Variables|Default|SetSelectedCard cardGuid))
      (Default|CallSelectedCardEvent _output_get)
      (else
        (Default|CallCardSelectFailedEvent cardGuid)
        (Development|PrintString "Not Enough Pips" true true "(R=0.782885,G=0.183969,B=1.000000,A=1.000000)")))))

(fn AddCard
  (params (CardName :type String) (CallAddCardEvent :type Boolean))
  (LocalVariables|SetcardGuid (Guid|NewGuid))
  (Utilities|Map|Add (Variables|Default|GetCardsInHand) (LocalVariables|GetcardGuid) (Class|KismetStringLibrary|ToUpper CardName))
  (if CallAddCardEvent
    (Default|CallAddCardEvent (LocalVariables|GetcardGuid) (CallFunction|CardNametoData CardName))))

(fn RemoveCard
  (params (Guid :type Guid%20Structure) (CallRemoveCardEvent :type Boolean))
  (if (== Guid (Variables|Default|GetSelectedCard))
    (CallFunction|DeselectCard (Variables|Default|GetSelectedCard) false))
  (Utilities|Map|Remove (Variables|Default|GetCardsInHand) Guid)
  (if CallRemoveCardEvent
    (Default|CallRemoveCardEvent Guid)))

(fn DeselectCard
  (params (cardGuid :type Guid%20Structure) (ReactivateMovement :type Boolean))
  (bind _gridmanager (Variables|Default|GetGridManager))
  (Default|CallDeselectedCardEvent cardGuid)
  (Variables|Default|SetSelectedCard "")
  (Variables|/Game/Systems/Grid/BP_GridManagerDataVersion.BP_GridManagerDataVersion_C|SetMovementMode _gridmanager false)
  (Default|DeselectExternalCells _gridmanager)
  (if ReactivateMovement
    (Default|ToggleMovemode (Variables|Default|GetGridManager) true)))

(fn UseCard
  (params (LocationToUseCard :type Int%20Vector%20Structure))
  (bind _gridmanager (Variables|Default|GetGridManager))
  (bind _gridmanager_2 (Variables|Default|GetGridManager))
  (bind _worldpos (Default|CellIndextoWorldPos _gridmanager_2 LocationToUseCard true false))
  (bind _cellinfo (Default|CellIndextoCellData _gridmanager LocationToUseCard))
  (bind _currentunit (Variables|/Game/Systems/Grid/BP_GridCell.BP_GridCell_C|GetCurrentUnit _cellinfo))
  (if (CallFunction|IsValidCard (Variables|Default|GetSelectedCard))
    (LocalVariables|SetTempCardData (CallFunction|CardGuidtoData (Variables|Default|GetSelectedCard)))
    (if (Utilities|IsValid _currentunit)
      (if (< (.carddamage (LocalVariables|GetTempCardData)) 0)
        (Default|Heal _currentunit (Math|Conversions|ToFloat(Integer) (Math|Integer|Absolute(Integer) (.carddamage (LocalVariables|GetTempCardData)))))
        (else
          (Default|Damage _currentunit (Math|Conversions|ToFloat(Integer) (.carddamage (LocalVariables|GetTempCardData)))))))
    (Default|UsePips (Variables|Default|GetCurrentUnit) (.pipcost (LocalVariables|GetTempCardData)))
    (Utilities|Array|RemoveItem (Variables|/Game/Units/BP_Unit.BP_Unit_C|GetcurrentRoundCardHand (Variables|Default|GetCurrentUnit)) (.Value (Utilities|Map|Find (Variables|Default|GetCardsInHand) (Variables|Default|GetSelectedCard))))
    (if (.removeonuse (LocalVariables|GetTempCardData))
      (CallFunction|RemoveCard (Variables|Default|GetSelectedCard) true)
      (Default|ToggleMovemode (Variables|Default|GetGridManager) true)
      (else
        (CallFunction|DeselectCard (Variables|Default|GetSelectedCard) true)))
    (for _array_element (.particlenames (LocalVariables|GetTempCardData))
      (Default|SpawnParticle (Variables|Default|GetCardParticalAndSoundManager) _array_element _worldpos (Math|Rotator|SelectRotator (Math|Rotator|FindLookatRotation (Transformation|GetActorLocation (Variables|Default|GetCurrentUnit)) _worldpos) "0, 0, 0" (.orientfx (LocalVariables|GetTempCardData)))))
    (for _array_element_2 (.cardsound (LocalVariables|GetTempCardData))
      (Default|PlaySound (Variables|Default|GetCardParticalAndSoundManager) _array_element_2 (Default|CellIndextoWorldPos (Variables|Default|GetGridManager) LocationToUseCard true false)))))

(fn IsValidCard
  (params (cardGuid :type Guid%20Structure))
  (return (and (Guid|IsValidGuid cardGuid) (Utilities|Map|Contains (Variables|Default|GetCardsInHand) cardGuid))))

(fn SelectUnit
  (params (Unit :type BP%20Unit%20Object%20Reference))
  (if (and (Utilities|IsValid (Variables|Default|GetCurrentUnit)) (!= (Variables|Default|GetCurrentUnit) Unit))
    (CallFunction|DeselectUnit)
    (CallFunction|UnbindUnitPipsUpdated (Variables|Default|GetCurrentUnit)))
  (if (Utilities|Enum|Equal(Enum) (Variables|/Game/Units/BP_Unit.BP_Unit_C|GetFaction Unit) "NewEnumerator0")
    (Default|CallSelectedUnitEvent 0 Unit)
    (CallFunction|BindUnitPipsUpdated Unit)
    (bind _output_get (Variables|Default|SetCurrentUnit Unit))
    (CallFunction|LoadHand (Variables|/Game/Units/BP_Unit.BP_Unit_C|GetcurrentRoundCardHand _output_get) true)
    (CallFunction|CheckCardAvalibility (Variables|/Game/Units/BP_Unit.BP_Unit_C|GetcurrentActionPips Unit))
    (Default|ToggleMovemode (Variables|Default|GetGridManager) true)))

(fn DeselectUnit
  (Utilities|IsValid (Variables|Default|GetCurrentUnit)
    (:Is%20Valid
      (Default|CallDeselectedUnitEvent (Variables|Default|GetCurrentUnit))
      (Variables|Default|SetCurrentUnit 0)
      (CallFunction|ClearHand))
    (:Is%20Not%20Valid
      (Development|PrintString "NO VALID UNIT TO DESELECT (card manager)" true true "(R=1.000000,G=0.000000,B=0.077781,A=1.000000)"))))

(fn CheckCardAvalibility
  (params (availablePips :type Integer))
  (bind _keys (Utilities|Map|Keys (Variables|Default|GetCardsInHand)))
  (for _array_element _keys
    (if (<= (.pipcost (CallFunction|CardGuidtoData _array_element)) availablePips)
      (Utilities|Array|Add (LocalVariables|GetavailableGUIDs) _array_element)
      (else
        (Utilities|Array|Add (LocalVariables|GetunavailableGUIDs) _array_element))))
  (Default|CallUpdateAvailableCardsEvent (LocalVariables|GetavailableGUIDs))
  (Default|CallUpdateUnavailableCardsEvent (LocalVariables|GetunavailableGUIDs)))

(fn DisplayCardRange
  (params (CardGuid :type Guid%20Structure))
  (bind _carddata (CallFunction|CardGuidtoData CardGuid))
  (bind _gridmanager (Variables|Default|GetGridManager))
  (bind _gridmanager_2 (Variables|Default|GetGridManager))
  (bind _gridmanager_3 (Variables|Default|GetGridManager))
  (CallFunction|DeselectCard)
  (Default|ToggleMovemode _gridmanager false)
  (bind _visitedmap (Class|PathFinder|DijkstraPathingFloodFill (Variables|/Script/Ultravile_Engine.GridManager|GetpathFinder _gridmanager) (Variables|/Script/Ultravile_Engine.GridCell|GetcellIndex (Variables|/Game/Systems/Grid/BP_GridManagerDataVersion.BP_GridManagerDataVersion_C|GetSelectedCell _gridmanager_2)) (.castrange _carddata) (Variables|/Game/Systems/Grid/BP_GridManagerDataVersion.BP_GridManagerDataVersion_C|GetGridCellsNonBP _gridmanager_2) false))
  (bind _keys (Utilities|Map|Keys _visitedmap))
  (bind _cellarray (Default|IndexArraytoCellArray (Variables|Default|GetGridManager) _keys))
  (bind _selectedgridcells (Default|FindOccupiedCellsinCollection _gridmanager_3 _cellarray (Utilities|Select :Index (.targettype _carddata) :FriendlyUnit (Utilities|Array|MakeArray "NewEnumerator1") :EnemyUnit (Utilities|Array|MakeArray "NewEnumerator2") :AllUnits (Utilities|Array|MakeArray "NewEnumerator2" "NewEnumerator1") :EmptyCell (Utilities|Array|MakeArray "NewEnumerator0") :AllCells (Utilities|Array|MakeArray "NewEnumerator3" "NewEnumerator1" "NewEnumerator2" "NewEnumerator0"))))
  (Default|SelectExternalCells _gridmanager_3 _selectedgridcells false true "(R=1.000000,G=1.000000,B=1.000000,A=1.000000)" "/Game/MaterialLibrary/GridUI/MI_Grid_Target.MI_Grid_Target")
  (Default|SelectExternalCells _gridmanager_3 _cellarray true false "(R=0.250000,G=0.250000,B=0.250000,A=1.000000)" "/Game/MaterialLibrary/GridUI/MI_Grid_Square.MI_Grid_Square"))

(fn CardGuidtoData
  (params (CardGuid :type Guid%20Structure))
  (return (CallFunction|CardNametoData (.Value (Utilities|Map|Find (Variables|Default|GetCardsInHand) CardGuid)))))

(fn CardNametoData
  (params (CardName :type String))
  (return (.Value (Utilities|Map|Find (Variables|Default|GetCardDictionary) (Class|KismetStringLibrary|ToUpper CardName)))))