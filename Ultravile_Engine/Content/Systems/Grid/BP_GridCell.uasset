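; BP_GridCell is a grid cell that tracks which unit stands on it and whether it is walkable.
; AddUnit links cell and unit both ways, derives the Occupyer state from the unit's faction, with Special sharing Enemy's value, and blocks walking.
; RemoveUnit clears both references and reopens the cell.
; SetAwaitingUnit blocks the cell with its own Occupyer state without assigning a unit.
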(fn AddUnit
  (params (Unit :type BP%20Unit%20Object%20Reference))
  (bind _output_get (Variables|Default|SetCurrentUnit Unit))
  (Variables|Default|SetOccupyer (Utilities|Select :Index (Variables|/Game/Units/BP_Unit.BP_Unit_C|GetFaction _output_get) :NewEnumerator0 "NewEnumerator1" :NewEnumerator1 "NewEnumerator2" :NewEnumerator3 "NewEnumerator2" :NewEnumerator2 "NewEnumerator3"))
  (Variables|/Game/Units/BP_Unit.BP_Unit_C|SetCurrentCell (Variables|Default|GetCurrentUnit) self)
  (Variables|Default|SetisWalkable false))

(fn RemoveUnit
  (Variables|Default|SetOccupyer "NewEnumerator0")
  (Variables|/Game/Units/BP_Unit.BP_Unit_C|SetCurrentCell (Variables|Default|GetCurrentUnit) 0)
  (Variables|Default|SetCurrentUnit 0)
  (Variables|Default|SetisWalkable true))

(fn SetAwaitingUnit
  (Variables|Default|SetOccupyer "NewEnumerator4")
  (Variables|Default|SetisWalkable false))