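; Turn manager for a grid-based tactics game, rotating rounds between friendly, enemy and special teams.
; On start it finds all units, snaps them to the grid manager's cells and sorts them by faction.
; It cycles selection through the active team, skipping finished or dead units, triggers enemy random moves, and advances the round when all finish.
; It also updates the turn UI and binds keys for cycling, completion and test damage/heal.
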(event EventBeginPlay
  (Utilities|FlowControl|Delay 0.1)
  (bind _returnvalue (Actor|GetActorOfClass "/Game/Systems/Grid/BP_GridManagerDataVersion.BP_GridManagerDataVersion_C"))
  (Utilities|IsValid _returnvalue
    (:Is%20Valid
      (Variables|Default|SetGridManager _returnvalue)
      (Variables|Default|SetcurrentGameState "NewEnumerator0")
      (CallFunction|FindAllUnits)
      (CallFunction|SortAllUnits)
      (Utilities|FlowControl|Delay 0.2)
      (CallFunction|BeginRound))))

(event Input|KeyboardEvents|H
  (params (Key :type Key%20Structure))
  (:Pressed
    (Default|Heal (Variables|Default|GetselectedUnit) 2.0)))

(event Input|KeyboardEvents|G
  (params (Key :type Key%20Structure))
  (:Pressed
    (Default|Damage (Variables|Default|GetselectedUnit) 2.0)))

(event Input|KeyboardEvents|SpaceBar
  (params (Key :type Key%20Structure))
  (:Pressed
    (CallFunction|CompleteRound)))

(event Input|KeyboardEvents|Tab
  (params (Key :type Key%20Structure))
  (:Pressed
    (switch Utilities|FlowControl|Switch|SwitchonEGameState (Variables|Default|GetcurrentGameState)
      (:NewEnumerator0
        (CallFunction|CycleUnit)))))

(event Input|KeyboardEvents|F
  (params (Key :type Key%20Structure))
  (:Pressed
    (CallFunction|CompleteTurn)))

(fn ConstructionScript)

(fn FindAllUnits
  (bind _gridmanager (Variables|Default|GetGridManager))
  (bind _outactors (Actor|GetAllActorsOfClass "/Game/Units/BP_Unit.BP_Unit_C"))
  (for _array_element _outactors
    (Utilities|Array|AddUnique (Variables|Default|GetallUnits) _array_element)
    ;[1 1 1] Temp to allign to grid
    (Transformation|SetWorldLocation (Variables|/Game/Units/BP_Unit.BP_Unit_C|GetBox%28Root%29 _array_element) (Default|CellIndextoWorldPos _gridmanager (Default|WorldPostoCellIndex _gridmanager (Transformation|GetWorldLocation (Variables|/Game/Units/BP_Unit.BP_Unit_C|GetBox%28Root%29 _array_element))) true false) false false)
    (Utilities|IsValid _array_element
      (:Is%20Valid
        (Default|AddUnit (Default|CellIndextoCellData (Variables|Default|GetGridManager) (Default|WorldPostoCellIndex _gridmanager (Transformation|GetWorldLocation (Variables|/Game/Units/BP_Unit.BP_Unit_C|GetBox%28Root%29 _array_element)))) _array_element)))))

(fn SortAllUnits
  (for _array_element (Variables|Default|GetallUnits)
    (switch Utilities|FlowControl|Switch|SwitchonEFaction (Variables|/Game/Units/BP_Unit.BP_Unit_C|GetFaction _array_element)
      (:NewEnumerator0
        (Utilities|Array|AddUnique (Variables|Default|GetfriendlyUnits) _array_element)
        (Variables|/Game/Units/BP_Unit.BP_Unit_C|SetIsVisable _array_element true))
      (:NewEnumerator1
        (Utilities|Array|AddUnique (Variables|Default|GetenemyUnits) _array_element))
      (:NewEnumerator3
        (Utilities|Array|AddUnique (Variables|Default|GetspecialUnits) _array_element :!label _label))
      (:NewEnumerator2
        (goto _label)))))

(fn CompleteTurn
  (bind _selectedunit (Variables|Default|GetselectedUnit))
  (Utilities|IsValid _selectedunit
    (:Is%20Valid
      (Default|CompleteTurn _selectedunit)
      (CallFunction|CycleUnit))))

(fn CompleteRound
  (bind _currentunitarray (Helper|GetCurrentUnitArray))
  (if (not (CallFunction|CheckifAnyUnitsAreBusy _currentunitarray))
    (Helper|ResetUnits _currentunitarray)
    (switch Utilities|FlowControl|Switch|SwitchonEGameState (Variables|Default|GetcurrentGameState)
      (:NewEnumerator0
        _)
      (:NewEnumerator1
        _)
      (:NewEnumerator4
        _))
    (Variables|Default|SetcurrentGameState (Utilities|Select :Index (Variables|Default|GetcurrentGameState) :NewEnumerator0 "NewEnumerator1" :NewEnumerator1 "NewEnumerator4" :NewEnumerator4 "NewEnumerator0"))
    (CallFunction|BeginRound)))

(fn BeginRound
  (switch Utilities|FlowControl|Switch|SwitchonEGameState (Variables|Default|GetcurrentGameState)
    (:NewEnumerator0
      (Development|PrintString "PlayeTeam" true true "(R=0.039774,G=0.385417,B=0.044011,A=1.000000)"))
    (:NewEnumerator1
      (Development|PrintString "EnemyTeam" true true "(R=0.406250,G=0.013698,B=0.086901,A=1.000000)"))
    (:NewEnumerator4
      (Development|PrintString "SpecialRound" true true "(R=0.627967,G=0.633333,B=0.106348,A=1.000000)")))
  (Helper|ResetUnits (Helper|GetCurrentUnitArray))
  (Variables|Default|SetcurrentUnitIndex 0)
  (CallFunction|CycleUnit)
  (CallFunction|SetRoundText))

(fn SelectUnit
  (params (Unit :type BP%20Unit%20Object%20Reference))
  (Utilities|IsValid (Variables|Default|GetselectedUnit)
    (:Is%20Valid
      (CallFunction|DeselectUnit))
    (:Is%20Not%20Valid
      _))
  (if (and (Utilities|Enum|Equal(Enum) (Variables|/Game/Units/BP_Unit.BP_Unit_C|GetFaction Unit) "NewEnumerator0") (not (Variables|/Game/Units/BP_Unit.BP_Unit_C|GetisMoving Unit)))
    (Default|SelectCell (Variables|Default|GetGridManager) (Variables|/Script/Ultravile_Engine.GridCell|GetcellIndex (Variables|/Game/Units/BP_Unit.BP_Unit_C|GetCurrentCell Unit))))
  (bind _output_get (Variables|Default|SetselectedUnit Unit))
  (Default|SelectUnit _output_get))

(fn CycleUnit
  (Variables|Default|SetcurrentUnitIndex (Utilities|CycleArrayIndex (Variables|Default|GetcurrentUnitIndex) (Helper|GetCurrentUnitArray)))
  (if (Utilities|Array|IsEmpty (Helper|GetCurrentUnitArray))
    (CallFunction|CompleteRound)
    (elif (or (Variables|/Game/Units/BP_Unit.BP_Unit_C|GetCompletedTurn (Helper|GetUnitwithIndex (Variables|Default|GetcurrentUnitIndex) (Helper|GetCurrentUnitArray))) (not (Variables|/Game/Units/BP_Unit.BP_Unit_C|GetIsAlive (Helper|GetUnitwithIndex (Variables|Default|GetcurrentUnitIndex) (Helper|GetCurrentUnitArray)))))
      (LocalVariables|SetAllCompleted true)
      (for _array_element (Helper|GetCurrentUnitArray)
        (if (not (or (Variables|/Game/Units/BP_Unit.BP_Unit_C|GetCompletedTurn _array_element) (not (Variables|/Game/Units/BP_Unit.BP_Unit_C|GetIsAlive _array_element))))
          (LocalVariables|SetAllCompleted false)))
      (if (LocalVariables|GetAllCompleted)
        (CallFunction|CompleteRound)
        (else
          (CallFunction|CycleUnit)))
      (else
        (CallFunction|SelectUnit (Helper|GetUnitwithIndex (Variables|Default|GetcurrentUnitIndex) (Helper|GetCurrentUnitArray)))
        (bind _asbp_unit_enemy (Utilities|Casting|CastToBP_Unit_Enemy (Helper|GetUnitwithIndex (Variables|Default|GetcurrentUnitIndex) (Helper|GetCurrentUnitArray))))
        (Default|RandomMove _asbp_unit_enemy)))))

(fn GetUnitwithIndex
  (params (Index :type Integer) (UnitArray :type Array%20of%20BP%20Unit%20Object%20References))
  (return (Utilities|Array|Get(acopy) UnitArray Index)))

(fn ResetUnits
  (params (Unit%20Array :type Array%20of%20BP%20Unit%20Object%20References))
  (for _array_element Unit%20Array
    (Default|RoundReset _array_element))
  (return))

(fn GetCurrentUnitArray
  (return (Utilities|Select :Index (Variables|Default|GetcurrentGameState) :NewEnumerator0 (Variables|Default|GetfriendlyUnits) :NewEnumerator1 (Variables|Default|GetenemyUnits) :NewEnumerator4 (Variables|Default|GetspecialUnits))))

(fn IsValidUnitIndex
  (params (Index :type Integer) (Unit%20Array :type Array%20of%20BP%20Unit%20Object%20References))
  (bind _returnvalue (Utilities|Array|Length Unit%20Array))
  (return (and (and (<= Index _returnvalue) (> Index -1)) (> _returnvalue 0))))

(fn DeselectUnit
  (Default|DeselectCell (Variables|Default|GetGridManager))
  (Default|DeselectUnit (Variables|Default|GetselectedUnit))
  (Variables|Default|SetselectedUnit 0))

(fn CheckifAnyUnitsAreBusy
  (params (Unit%20Array :type Array%20of%20BP%20Unit%20Object%20References))
  (LocalVariables|SetUnitsAreBusy false)
  (for _array_element Unit%20Array
    (if (Default|IsBusy _array_element)
      (LocalVariables|SetUnitsAreBusy true)))
  (return (LocalVariables|GetUnitsAreBusy)))

(fn RemoveUnit
  (params (Unit :type BP%20Unit%20Object%20Reference))
  (Default|RemoveUnit (Variables|/Game/Units/BP_Unit.BP_Unit_C|GetCurrentCell Unit))
  (Utilities|Array|RemoveItem (Utilities|Select :Index (Variables|/Game/Units/BP_Unit.BP_Unit_C|GetFaction Unit) :NewEnumerator0 (Variables|Default|GetfriendlyUnits) :NewEnumerator1 (Variables|Default|GetenemyUnits) :NewEnumerator3 (Variables|Default|GetspecialUnits) :NewEnumerator2 0) Unit)
  (Utilities|Array|RemoveItem (Variables|Default|GetallUnits) Unit)
  (if (== Unit (Variables|Default|GetselectedUnit))
    (CallFunction|CycleUnit)))

(fn SetRoundText
  (bind _foundwidgets (Widget|GetAllWidgetsOfClass "/Game/UI/W_GameUI.W_GameUI_C" true))
  (Rendering|Components|TextRender|SetText (Variables|/Game/UI/W_GameUI.W_GameUI_C|GetCurrentTurn (Utilities|Array|Get(acopy) _foundwidgets)) (Utilities|Select :Index (Variables|Default|GetcurrentGameState) :NewEnumerator0 "Friendly Turn" :NewEnumerator1 "Enemy Turn" :NewEnumerator4 "Special Turn"))
  (Appearance|SetColorandOpacity (Variables|/Game/UI/W_GameUI.W_GameUI_C|GetCurrentTurn (Utilities|Array|Get(acopy) _foundwidgets)) (Utilities|Struct|MakeSlateColor (Utilities|Select :Index (Variables|Default|GetcurrentGameState) :NewEnumerator0 "(R=0.103082,G=0.791667,B=0.139882,A=1.000000)" :NewEnumerator1 "(R=0.885417,G=0.170626,B=0.170626,A=1.000000)" :NewEnumerator4 "(R=0.645833,G=0.588528,B=0.121094,A=1.000000)")) :!class /Script/UMG.TextBlock))