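; Base unit for a turn-based, grid-and-card tactics game, with faction, health, movement range and action pips.
; Movement steps along a grid path via a timeline, spending range then pips and updating cell occupancy through the grid manager.
; Damage drives a delayed health-bar timeline, and death removes the unit from the turn manager.
; Selection switches to the nearest camera found at start, focuses it and notifies the card manager.
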(event Custom|Move
  (params (Positions :type Array%20of%20Vectors))
  (bind _gridmanager (Variables|Default|GetGridManager))
  (bind _gridmanager_2 (Variables|Default|GetGridManager))
  ;[1 1 1] Movement
  (if (and (> (Utilities|Array|Length Positions) 1) (Variables|Default|GetisMoving)) :!label _label
    (Default|RemoveUnit (Variables|Default|GetCurrentCell))
    (Components|Timeline|SetPlayRate (Variables|Default|GetTimeline_0) (Variables|Default|GetMoveAnimationSpeed))
    (bind _value (Utilities|QueuePop Positions))
    (bind _value_2 (Utilities|QueuePeak Positions))
    (bind _movetrack (Timeline|Timeline_0 PlayFromStart)
      (:Update
        (Transformation|SetWorldLocation (Variables|Default|GetBox%28Root%29) (Math|Vector|Lerp(Vector) _value _value_2 _movetrack) true false))
      (:Finished
        (Default|AddUnit (Default|CellIndextoCellData _gridmanager (Default|WorldPostoCellIndex _gridmanager _value_2)) self)
        (if (> (Variables|Default|GetMovementRange) 0)
          (Math|Integer|DecrementInt (Variables|Default|GetMovementRange)
            (:%20%20
              (CallFunction|UpdateStats)))
          (elif (> (Variables|Default|GetcurrentActionPips) 0)
            (CallFunction|UsePips 1)))
        (if (and (<= (Variables|Default|GetMovementRange) 0) (<= (Variables|Default|GetcurrentActionPips) 0))
          (Variables|Default|SetisMoving false)
          (goto _label)
          (else
            (goto _label)))))
    (else
      (bind _value_3 (Utilities|QueuePop Positions))
      (Default|AddUnit (Default|CellIndextoCellData _gridmanager_2 (Default|WorldPostoCellIndex _gridmanager_2 _value_3)) self)
      (Variables|Default|SetisMoving false)
      (if (Variables|Default|GetisSelected)
        (Default|SelectUnit (Variables|Default|GetTurnManager) self)
        (CallFunction|TestTurnCompletion)
        (else
          (CallFunction|TestTurnCompletion))))))

(event Custom|Set%20Default%20Camera
  (bind _outactors (Actor|GetAllActorsOfClass "/Game/Systems/Camera/BP_CameraCollider.BP_CameraCollider_C"))
  (bind _output_get (Variables|Default|SetAll%20Cameras _outactors))
  (for _array_element _output_get
    (Utilities|Array|Add (Variables|Default|GetCamera%20Distances) (Math|Vector|Distance(Vector) (Transformation|GetWorldLocation (Variables|/Game/Systems/Camera/BP_CameraCollider.BP_CameraCollider_C|GetDefaultSceneRoot _array_element)) (Transformation|GetWorldLocation (Variables|Default|GetBox%28Root%29)))))
  (bind _output_get_2 (Variables|Default|SetCurrent%20Camera (Utilities|Array|Get(acopy) (Variables|Default|GetAll%20Cameras) (.IndexOfMinValue (Math|Float|MinOfFloatArray (Variables|Default|GetCamera%20Distances))))))
  (Default|SwitchCamera _output_get_2))

(event EventHeal
  (params (HealAmount :type Float%20%28double-precision%29))
  (bind _health (Variables|Default|GetHealth))
  (bind _returnvalue (+ _health HealAmount))
  (if (> _returnvalue (Variables|Default|GetMaxHealth))
    (CallFunction|UpdateHealth (Variables|Default|GetMaxHealth))
    (else
      (CallFunction|UpdateHealth _returnvalue))))

(event EventDamage
  (params (DamageAmount :type Float%20%28double-precision%29))
  (bind _health (Variables|Default|GetHealth))
  (bind _returnvalue (- _health DamageAmount))
  (if (or (<= (Variables|Default|GetDelayedHealth) (Variables|Default|GetHealth)) (Variables|Default|GetDelayHealthRunning))
    (Variables|Default|SetDelayedHealth (Math|Float|SelectFloat (Variables|Default|GetDelayedHealthTimelineValue) _health (Variables|Default|GetDelayHealthRunning)))
    (Variables|Default|SetDelayHealthRunning false))
  (if (<= _returnvalue 0.0)
    (CallFunction|UpdateHealth 0.0)
    (CallFunction|Die)
    (bind _delaytrackstart (Timeline|DelayedTrack PlayFromStart)
      (:Update
        (if (> _delaytrackstart 0.0)
          (Variables|Default|SetDelayHealthRunning true))
        (Variables|Default|SetDelayedHealthTimelineValue (Math|Float|Lerp (Variables|Default|GetDelayedHealth) (Variables|Default|GetHealth) _delaytrackstart))
        (Default|CallHealthDelayedUpdated (Math|Float|Lerp (Variables|Default|GetDelayedHealth) (Variables|Default|GetHealth) _delaytrackstart) (Variables|Default|GetMaxHealth)))
      (:Finished
        (Variables|Default|SetDelayedHealth (Variables|Default|GetHealth))
        (Variables|Default|SetDelayHealthRunning false)))
    (else
      (CallFunction|UpdateHealth _returnvalue)
      (Timeline|DelayedTrack PlayFromStart))))

(event EventDie
  (Variables|Default|SetIsAlive false)
  (Default|RemoveUnit (Variables|Default|GetTurnManager) self)
  (Utilities|FlowControl|Delay 3.0)
  (Actor|DestroyActor))

(event EventBeginPlay
  (CallFunction|SetDefaultCamera)
  (bind _returnvalue (Actor|GetActorOfClass "/Game/Systems/Grid/BP_GridManagerDataVersion.BP_GridManagerDataVersion_C"))
  (Variables|Default|SetGridManager _returnvalue)
  (bind _returnvalue_2 (Actor|GetActorOfClass "/Game/Systems/TurnManager/BP_TurnManager.BP_TurnManager_C"))
  (Variables|Default|SetTurnManager _returnvalue_2)
  (Variables|Default|SetHealth (Variables|Default|GetMaxHealth))
  ;[1 1 1] Health UI Setup
  (bind _asw_health (Utilities|Casting|CastToW_Health (UserInterface|GetWidget (Variables|Default|GetHealthBarWidget))))
  (Default|Setup _asw_health self (Utilities|Select :Index (Variables|Default|GetFaction) :NewEnumerator0 "(R=0.099609,G=0.708333,B=0.172737,A=1.000000)" :NewEnumerator1 "(R=0.838542,G=0.161594,B=0.161594,A=1.000000)" :NewEnumerator3 "(R=0.781250,G=0.731364,B=0.250529,A=1.000000)" :NewEnumerator2 "(R=0.500000,G=0.500000,B=0.500000,A=1.000000)"))
  (CallFunction|UpdateHealth (Variables|Default|GetMaxHealth))
  (Default|CallMaxHealthUpdated (Variables|Default|GetMaxHealth)))

(event Input|KeyboardEvents|Z
  (params (Key :type Key%20Structure))
  (:Pressed
    (CallFunction|AddStatusUI)))

(fn ConstructionScript
  (Rendering|Material|SetMaterial (Variables|Default|GetSkeletalMesh) 0 (Utilities|Select :Index (Variables|Default|GetFaction) :NewEnumerator0 "/Game/Units/MI_UnitDebug_Friendly.MI_UnitDebug_Friendly" :NewEnumerator1 "/Game/Units/MI_UnitDebug_Enemy.MI_UnitDebug_Enemy" :NewEnumerator3 "/Game/Units/MI_UnitDebug_Special.MI_UnitDebug_Special" :NewEnumerator2 "/Game/Characters/Mannequins/Materials/Instances/Quinn/MI_Quinn_01.MI_Quinn_01"))
  (bind _returnvalue (Actor|GetActorOfClass "/Game/Systems/CardSystem/BP_CardManager.BP_CardManager_C"))
  (Variables|Default|SetCardManager _returnvalue))

(fn RoundReset
  (Variables|Default|SetCompletedTurn false)
  (Variables|Default|SetMovementRange (Variables|Default|GetDefualtMovementRange))
  (Variables|Default|SetcurrentActionPips (Variables|Default|GetmaxActionPips))
  (CallFunction|UpdatePipUI)
  (Variables|Default|SetcurrentRoundCardHand (Variables|Default|GetCardHand)))

(fn SelectUnit
  (if (Variables|Default|GetIsVisable)
    (CallFunction|SwitchCamera)
    (bind _asbp_camera_pawn (Utilities|Casting|CastToBP_CameraPawn (Game|Player|GetPlayerPawn 0)))
    (Variables|/Script/CinematicCamera.CineCameraComponent|SetFocusSettings (Variables|/Game/Systems/Camera/BP_CameraPawn.BP_CameraPawn_C|GetCineCamera _asbp_camera_pawn) (Utilities|Struct|MakeCameraFocusSettings "Tracking" 1e+05 (Utilities|Struct|MakeCameraTrackingFocusSettings (Utilities|ResolveSoftReference self) "0.000000,0.000000,150.000000" false)))
    (Variables|/Game/Systems/Camera/BP_CameraPawn.BP_CameraPawn_C|SetTarget _asbp_camera_pawn self))
  (Variables|Default|SetisSelected true)
  (CallFunction|ShowUI true)
  (Default|SelectUnit (Variables|Default|GetCardManager) self)
  (Rendering|SetCustomDepthStencilValue (Variables|Default|GetSkeletalMesh) 1)
  (CallFunction|UpdatePipUI)
  (CallFunction|UpdateStats)
  (switch Utilities|FlowControl|Switch|SwitchonEFaction (Variables|Default|GetFaction)))

(fn DeselectUnit
  (Variables|Default|SetisSelected false)
  (CallFunction|ShowUI false)
  (Rendering|SetCustomDepthStencilValue (Variables|Default|GetSkeletalMesh) 0)
  (Default|DeselectUnit (Variables|Default|GetCardManager)))

(fn CompleteTurn
  (Variables|Default|SetCompletedTurn true))

(fn SwitchCamera
  (Default|SwitchCamera (Variables|Default|GetCurrent%20Camera)))

(fn MoveUnit
  (params (GridIndexPath :type Array%20of%20Int%20Vector%20Structures) (TargetCell :type Int%20Vector%20Structure))
  (bind _gridmanager (Variables|Default|GetGridManager))
  (bind _currentcell (Variables|Default|GetCurrentCell))
  (bind _cellindex (Variables|/Script/Ultravile_Engine.GridCell|GetcellIndex _currentcell))
  (Default|SetAwaitingUnit (Default|CellIndextoCellData (Variables|Default|GetGridManager) TargetCell))
  (if (Utilities|Array|ContainsItem GridIndexPath _cellindex)
    _
    (else
      (Utilities|Array|Insert GridIndexPath _cellindex)))
  (Variables|Default|SetisMoving true)
  (Default|DeselectCell _gridmanager)
  (CallFunction|Move (Default|CellIndexstoWorldPositions _gridmanager GridIndexPath true false true)))

(fn TestTurnCompletion
  (if (Utilities|Enum|Equal(Enum) (Variables|Default|GetFaction) "NewEnumerator1")
    (Default|CompleteTurn (Variables|Default|GetTurnManager))))

(fn IsAvailable
  (return (and (or (> (Variables|Default|GetcurrentActionPips) 0) (> (Variables|Default|GetMovementRange) 0)) (Variables|Default|GetIsAlive))))

(fn GetMaxMovementRange
  (return (Variables|Default|GetMovementRange)))

(fn IsBusy
  (return (Variables|Default|GetisMoving)))

(fn UpdateHealth
  (params (HealthAmount :type Float%20%28double-precision%29))
  (CallFunction|UpdateStats)
  (bind _output_get (Variables|Default|SetHealth HealthAmount))
  (if (< (Variables|Default|GetDelayedHealth) (Variables|Default|GetHealth))
    (Variables|Default|SetDelayedHealth (Variables|Default|GetHealth)))
  (Default|CallHealthUpdated _output_get (Variables|Default|GetMaxHealth)))

(fn ShowUI
  (params (Show :type Boolean)))

(fn UsePips
  (params (amountOfPips :type Integer))
  (bind _output_get (Variables|Default|SetcurrentActionPips (- (Variables|Default|GetcurrentActionPips) amountOfPips)))
  (if (< _output_get 0)
    (Variables|Default|SetcurrentActionPips 0))
  (CallFunction|UpdatePipUI)
  (Default|CallPipsUpdated (Variables|Default|GetcurrentActionPips)))

(fn UpdatePipUI
  (bind _currentactionpips (Variables|Default|GetcurrentActionPips))
  (bind _asw_health (Utilities|Casting|CastToW_Health (UserInterface|GetWidget (Variables|Default|GetHealthBarWidget))))
  (Rendering|Components|TextRender|SetText (Variables|/Game/UI/Unit/W_Health.W_Health_C|GetPipCount _asw_health) (Utilities|Text|ToText(Integer) _currentactionpips))
  (bind _foundwidgets (Widget|GetAllWidgetsOfClass "/Game/UI/W_GameUI.W_GameUI_C" true))
  (Rendering|Components|TextRender|SetText (Variables|/Game/UI/W_GameUI.W_GameUI_C|GetPipText (Utilities|Array|Get(acopy) _foundwidgets)) (Utilities|Text|ToText(String) (Utilities|String|Append "<img id=\"pip\"></> " (Utilities|String|Append (Utilities|String|Append "<GameUI>" (Utilities|String|ToString(Integer) _currentactionpips)) "</>")))))

(fn UpdateStats
  (bind _foundwidgets (Widget|GetAllWidgetsOfClass "/Game/UI/W_GameUI.W_GameUI_C" true))
  (if (not (Utilities|Array|IsEmpty _foundwidgets))
    (Rendering|Components|TextRender|SetText (Variables|/Game/UI/W_GameUI.W_GameUI_C|GetStatText (Utilities|Array|Get(acopy) _foundwidgets)) (Utilities|Text|ToText(String) (Utilities|String|Append (Utilities|String|Append (Utilities|String|Append " <img id=\"shield\"></>" (Utilities|String|Append (Utilities|String|Append "<GameUI>" "0") "</>")) (Utilities|String|Append " <img id=\"heart\"></>" (Utilities|String|Append (Utilities|String|Append "<GameUI>" (Utilities|String|ToString(Integer) (Math|Float|Truncate (Variables|Default|GetHealth)))) "</>"))) (Utilities|String|Append " <img id=\"boot\"></>" (Utilities|String|Append (Utilities|String|Append "<GameUI>" (Utilities|String|ToString(Integer) (Variables|Default|GetMovementRange))) "</>")))))))

(fn AddStatusUI
  (bind _asw_health (Utilities|Casting|CastToW_Health (UserInterface|GetWidget (Variables|Default|GetHealthBarWidget))))
  (for _array_element (Variables|Default|GetTestStatus)
    (Default|AddEffect _asw_health _array_element)))