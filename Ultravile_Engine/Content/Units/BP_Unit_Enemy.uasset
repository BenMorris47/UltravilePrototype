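; Enemy unit for grid-based movement that wanders to a random reachable cell when told to move.
; RandomMove triggers the moveRandom event, which waits briefly, then runs the GridManager pathfinder's Dijkstra flood fill over walkable cells within MovementRange.
; It removes the current cell from the results, picks one at random and has the GridManager move the unit there.
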(event Custom|moveRandom
  (bind _currentcell (Variables|Default|GetCurrentCell))
  (bind _gridmanager (Variables|Default|GetGridManager))
  (bind _cellindex (Variables|/Script/Ultravile_Engine.GridCell|GetcellIndex _currentcell))
  (Utilities|FlowControl|Delay 1.0)
  (bind _returnvalue (Class|PathFinder|DijkstraPathingFloodFill (Variables|/Script/Ultravile_Engine.GridManager|GetpathFinder _gridmanager) _cellindex (Variables|Default|GetMovementRange) (Variables|/Game/Systems/Grid/BP_GridManagerDataVersion.BP_GridManagerDataVersion_C|GetGridCellsNonBP _gridmanager) true))
  (Utilities|Array|RemoveItem _returnvalue _cellindex)
  (Default|MoveUnittoLocation (Variables|Default|GetGridManager) (.OutItem (Utilities|Array|Random _returnvalue)) self))

(event EventBeginPlay
  (|CallParentFunction))

(event Collision|EventActorBeginOverlap
  (params (OtherActor :type Actor%20Object%20Reference))
  (|CallParentFunction OtherActor) ; This node is disabled and will not be called.\nDrag off pins to build functionality.
)

(event EventTick
  (params (DeltaSeconds :type Float%20%28single-precision%29))
  (|CallParentFunction DeltaSeconds) ; This node is disabled and will not be called.\nDrag off pins to build functionality.
)

(fn ConstructionScript
  (|CallParentFunction))

(fn RandomMove
  (CallFunction|MoveRandom))