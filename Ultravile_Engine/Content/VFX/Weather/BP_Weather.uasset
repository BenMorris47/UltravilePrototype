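; BP_Weather is a weather actor that drives a rain particle effect and the related sky and rain material parameters.
; UpdateRain, run from construction and BeginPlay, moves a scene capture to the bounding box offset and feeds lifetime, box and SunRain-scaled spawn rate to the particles.
; It also writes SunRain and the capture's world height to material parameter collections.
; Calls to update the sky and wind Blueprints exist but never run.
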(event Custom|Update%20Rain
  (bind _sun_rain (Variables|Default|GetSun/Rain))
  (bind _rain (Variables|Default|GetRain))
  (Transformation|SetRelativeLocation (Variables|Default|GetSceneCaptureComponent2D) (Variables|Default|GetBounding%20Box%20Offset) false false) ; Syncs capture component to top of bounding box
  ;[1 1 1] Sets particle variables based on blueprint variables
  (Niagara|SetNiagaraVariable(Float) _rain "Lifetime" (Variables|Default|GetLifetime))
  (Niagara|SetNiagaraVariable(Float) _rain "Spawn Rate" (* (Variables|Default|GetRain%20Spawn%20Rate) _sun_rain))
  (Niagara|SetNiagaraVariable(Vector3) _rain "Bounding Box Size" (Variables|Default|GetBounding%20Box%20Size))
  (Niagara|SetNiagaraVariable(Vector3) _rain "Box Offset" (Variables|Default|GetBounding%20Box%20Offset))
  ;[1 1 1] Set material properties based on blueprint variables
  (Rendering|Material|SetScalarParameterValue "/Rain_Sky_BETA/Sky/MPC_Sky.MPC_Sky" "Sun/Rain" _sun_rain :!class /Script/Engine.KismetMaterialLibrary)
  (Rendering|Material|SetScalarParameterValue "/Game/VFX/Weather/Rain/MPC_Rain.MPC_Rain" "Height" (.z (Transformation|GetWorldLocation (Variables|Default|GetSceneCaptureComponent2D))) :!class /Script/Engine.KismetMaterialLibrary))

(event EventBeginPlay
  (CallFunction|UpdateRain))

(fn ConstructionScript
  (CallFunction|UpdateRain))