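; BP_Wind is a weather actor that drives global wind for materials and bends rain to match it.
; UpdateWind writes the actor's yaw and its intensity, noise size and speed variables into the MPC_Wind parameter collection.
; It also adds a yaw-based wind vector to BP_Weather's base rain velocity on the Rain effect.
; Updates run only on construction and BeginPlay, and require a valid BP_Weather reference.
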(event Custom|Update%20Wind
  (bind _wind_intensity (Variables|Default|GetWind%20Intensity))
  (bind _defaultsceneroot (Variables|Default|GetDefaultSceneRoot))
  (bind _returnvalue (Transformation|GetWorldRotation _defaultsceneroot))
  (bind _returnvalue_2 (Math|Trig|DegreesToRadians (.yaw _returnvalue)))
  (bind _asbp_weather (Utilities|Casting|CastToBP_Weather (Variables|Default|GetWeather%20BP)))
  ;[1 1 1] Sets material properties based on blueprint variables
  (Rendering|Material|SetScalarParameterValue "/Game/VFX/Weather/Wind/MPC_Wind.MPC_Wind" "Wind Direction (Degrees)" (+ (.yaw _returnvalue) 1.8e+02) :!class /Script/Engine.KismetMaterialLibrary)
  (Rendering|Material|SetScalarParameterValue "/Game/VFX/Weather/Wind/MPC_Wind.MPC_Wind" "Global Non-Dir Wind Intensity" (Variables|Default|GetNon-Dir%20Wind%20Intensity) :!class /Script/Engine.KismetMaterialLibrary)
  (Rendering|Material|SetScalarParameterValue "/Game/VFX/Weather/Wind/MPC_Wind.MPC_Wind" "Global Wind Intensity" (Variables|Default|GetWind%20Intensity) :!class /Script/Engine.KismetMaterialLibrary)
  (Rendering|Material|SetScalarParameterValue "/Game/VFX/Weather/Wind/MPC_Wind.MPC_Wind" "Global Wind Noise Size" (Variables|Default|GetWind%20Noise%20Size) :!class /Script/Engine.KismetMaterialLibrary)
  (Rendering|Material|SetScalarParameterValue "/Game/VFX/Weather/Wind/MPC_Wind.MPC_Wind" "Global Wind Speed" (Variables|Default|GetWind%20Speed) :!class /Script/Engine.KismetMaterialLibrary)
  (Niagara|SetNiagaraVariable(Vector3) (Variables|/Game/VFX/Weather/BP_Weather.BP_Weather_C|GetRain _asbp_weather) "Velocity" (+ (Math|Vector|MakeVector (* (* _wind_intensity (Math|Trig|Cos(Radians) _returnvalue_2)) 4e+01) (* (* _wind_intensity (Math|Trig|Sin(Radians) _returnvalue_2)) 4e+01) 0.0) (Variables|/Game/VFX/Weather/BP_Weather.BP_Weather_C|GetBase%20Rain%20Velocity _asbp_weather)) :!pinned true) ; Wind effects rain direction
)

(event EventBeginPlay
  (CallFunction|UpdateWind))

(fn ConstructionScript
  (CallFunction|UpdateWind))